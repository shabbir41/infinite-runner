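; BP_mainplayer is the player character for what appears to be a lane-based auto-runner.
; Tick constantly pushes it along world +X, scaled by Speed.
; Jump input uses the built-in jump, while Down only toggles the Slide flag.
; Left and right inputs snap the actor sideways by a fixed lane offset with a slight forward nudge, gated by Y-position bounds instead of a tracked lane index.
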(event EventTick
  (params (DeltaSeconds :type Float%20%28single-precision%29))
  ;[1 1 1] Movements
  (Pawn|Input|AddMovementInput (Math|Vector|GetForwardVector "0, 0, 0") (Variables|Default|GetSpeed) false))

(event Input|ActionEvents|InputActionJump
  (params (Key :type Key%20Structure :default "None"))
  ;[1 1 1] Actions
  (:Pressed
    (Character|Jump))
  (:Released
    (Character|StopJumping)))

(event Input|ActionEvents|InputActionDown
  (params (Key :type Key%20Structure :default "None"))
  ;[1 1 1] Actions
  (:Pressed
    (Variables|Default|Setslide? true))
  (:Released
    (Variables|Default|Setslide? false)))

(event Input|ActionEvents|InputActionMoveLeft
  (params (Key :type Key%20Structure :default "None"))
  (bind _returnvalue (Transformation|GetActorLocation))
  ;[1 1 1] Movements
  (:Pressed
    (if (> (.y _returnvalue) -175.0)
      (Transformation|SetActorLocation (Math|Vector|MakeVector (+ (.x _returnvalue) 15.0) (- (.y _returnvalue) 225.0) (.z _returnvalue)) false false))))

(event Input|ActionEvents|InputActionMoveRight
  (params (Key :type Key%20Structure :default "None"))
  (bind _returnvalue (Transformation|GetActorLocation))
  ;[1 1 1] Movements
  (:Pressed
    (if (< (.y _returnvalue) 175.0)
      (Transformation|SetActorLocation (Math|Vector|MakeVector (+ (.x _returnvalue) 15.0) (+ (.y _returnvalue) 225.0) (.z _returnvalue)) false true))))

(event Input|ActionEvents|InputActionJump
  (params (Key :type Key%20Structure :default "None")))

(fn ConstructionScript)