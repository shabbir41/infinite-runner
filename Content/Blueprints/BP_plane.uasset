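; BP_plane is a self-chaining ground segment that populates itself with obstacles, apparently for an endless-runner style level.
; On BeginPlay it repeatedly calls SpawnEnemy, which places BP_Obstacle actors using three marker components picked at random, with a random forward offset along world X.
; Any overlap with its Trigger spawns another BP_plane at the Arrow component's transform, extending the track.
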(event OnComponentBeginOverlap(Trigger)
  (params (OverlappedComponent :type Primitive%20Component%20Object%20Reference) (OtherActor :type Actor%20Object%20Reference) (OtherComp :type Primitive%20Component%20Object%20Reference) (OtherBodyIndex :type Integer) (bFromSweep :type Boolean) (SweepResult :type Hit%20Result%20Structure%20%28by%20ref%29))
  (Game|SpawnActorfromClass "BP_plane_C" (Transformation|GetWorldTransform (Variables|Default|GetArrow)) "AlwaysSpawn" 0 0))

(event EventBeginPlay
  (for _index (range 0 5)
    (CallFunction|SpawnEnemy)))

(event Collision|EventActorBeginOverlap
  (params (OtherActor :type Actor%20Object%20Reference)))

(event EventTick
  (params (DeltaSeconds :type Float%20%28single-precision%29)))

(fn ConstructionScript)

(fn SpawnEnemy
  (bind _returnvalue (Math|Random|RandomInteger 3))
  (bind _enemypos1 (Variables|Default|GetEnemyPos1))
  (bind _enemypos2 (Variables|Default|GetEnemyPos2))
  (bind _enemypos3 (Variables|Default|GetEnemyPos3))
  (bind _array (Utilities|Array|MakeArray _enemypos1 _enemypos2 _enemypos3))
  (bind _output (Utilities|Array|Get(acopy) _array _returnvalue))
  (bind _returnvalue_2 (Transformation|GetWorldLocation _output))
  (Game|SpawnActorfromClass "/Game/Enemies/BP_Obstacle.BP_Obstacle_C" (Math|Transform|MakeTransform (Math|Vector|MakeVector (+ (.x _returnvalue_2) (Math|Random|RandomFloatinRange 0.0 3e+03)) (.y _returnvalue_2) (.z _returnvalue_2)) "0, 0, 0" "1.000000,1.000000,1.000000") "Undefined" 0 0))